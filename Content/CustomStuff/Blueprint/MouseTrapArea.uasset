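; MouseTrapArea is a placement spot that snaps an actor tagged "mousetrap" into position when it enters the Box trigger.
; On overlap it teleports that actor to the area's location and sets its GrabComponent's GrabType to the enum's first entry.
; It then clears its own MouseTrap static mesh, which the construction script scales down uniformly.
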(event OnComponentBeginOverlap(Box)
  (params (OverlappedComponent :type Primitive%20Component%20Object%20Reference) (OtherActor :type Actor%20Object%20Reference) (OtherComp :type Primitive%20Component%20Object%20Reference) (OtherBodyIndex :type Integer) (bFromSweep :type Boolean) (SweepResult :type Hit%20Result%20Structure%20%28by%20ref%29))
  (if (Actor|ActorHasTag OtherActor "mousetrap")
    (Transformation|SetActorLocation OtherActor (Transformation|GetActorLocation) false true)
    (Variables|/Game/VRTemplate/Blueprints/GrabComponent.GrabComponent_C|SetGrabType (Actor|GetComponentbyClass OtherActor "/Game/VRTemplate/Blueprints/GrabComponent.GrabComponent_C") "NewEnumerator0")
    (Components|StaticMesh|SetStaticMesh (Variables|Default|GetMouseTrap) 0)))

(fn ConstructionScript
  (Transformation|SetWorldScale3D (Variables|Default|GetMouseTrap) "0.060000,0.060000,0.060000"))