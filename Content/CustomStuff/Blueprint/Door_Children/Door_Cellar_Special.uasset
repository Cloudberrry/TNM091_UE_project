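; Cellar door Blueprint that swings to follow a grab component, apparently on its handle.
; While the grab component is valid, Tick yaws the door from its look-at rotation, clamped to a 90-degree arc relative to the frame.
; Otherwise it snaps shut when near zero world yaw; dropping returns the handle collision to the handle location.
; The lock check clears Locked on both branches, so the door never stays locked.
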(event OnDropped(GrabComponent)
  (Transformation|SetWorldLocation (Variables|Default|GetHandleCollision) (Transformation|GetWorldLocation (Variables|Default|GetDoorHandleLocation)) false false))

(event EventTick
  (params (DeltaSeconds :type Float%20%28single-precision%29))
  (bind _door (Variables|Default|GetDoor))
  (bind _doorframe (Variables|Default|GetDoorFrame))
  (bind _grabcomponent (Variables|Default|GetGrabComponent))
  (bind _returnvalue (Transformation|GetWorldRotation _doorframe))
  (Utilities|FlowControl|Sequence
    (:then_0
      ;[1 1 1] Locked?
      (if (Math|Float|NearlyEqual(Float) (.yaw (Transformation|GetWorldRotation (Variables|Default|GetDoor))) 0.0 1e-06)
        (Variables|Default|SetLocked false)
        (else
          (Variables|Default|SetLocked false))))
    (:then_1
      (if (not (Variables|Default|GetLocked))
        (Utilities|IsValid _grabcomponent
          (:Is%20Valid
            (Transformation|SetWorldRotation _door (Math|Rotator|MakeRotator 0.0 0.0 (Math|Float|ClampAngle (- (.yaw (Math|Rotator|FindLookatRotation (Transformation|GetWorldLocation _grabcomponent) (Transformation|GetWorldLocation _door))) 0.0) (+ (.yaw _returnvalue) -9e+01) (+ (.yaw _returnvalue) 0.0))) false false))
          (:Is%20Not%20Valid
            (if (Math|Float|NearlyEqual(Float) (.yaw (Transformation|GetWorldRotation _door)) 0.0 1e+01)
              (Transformation|SetWorldRotation _door "0, 0, 0" false false))))))))

(fn ConstructionScript)