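; BP_Holster is a holster actor that stores one flashlight-tagged item when that item overlaps its HolsterMesh.
; If empty, it flags the item's GrabComponent as holstered, passes itself as the holster, teleports the item to the mesh and attaches it.
; Nothing here clears HasItem; CanHold only resets a DoOnce after a short delay, and a Swedish note says something stopped working.
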(event OnComponentBeginOverlap(HolsterMesh)
  (params (OverlappedComponent :type Primitive%20Component%20Object%20Reference) (OtherActor :type Actor%20Object%20Reference) (OtherComp :type Primitive%20Component%20Object%20Reference) (OtherBodyIndex :type Integer) (bFromSweep :type Boolean) (SweepResult :type Hit%20Result%20Structure%20%28by%20ref%29))
  (if (Actor|ActorHasTag OtherActor "flashlight")
    (if (not (Variables|Default|GetHasItem))
      (bind _output_get (Variables|Default|SetHolsteredItem OtherActor))
      (Variables|/Game/VRTemplate/Blueprints/GrabComponent.GrabComponent_C|SetIsHolstered (Actor|GetComponentbyClass _output_get "/Game/VRTemplate/Blueprints/GrabComponent.GrabComponent_C") true)
      (Variables|/Game/VRTemplate/Blueprints/GrabComponent.GrabComponent_C|SetHolster (Actor|GetComponentbyClass _output_get "/Game/VRTemplate/Blueprints/GrabComponent.GrabComponent_C") self)
      (Transformation|SetActorLocation (Variables|Default|GetHolsteredItem) (Transformation|GetWorldLocation (Variables|Default|GetHolsterMesh)) false true)
      (Transformation|AttachActorToActor (Variables|Default|GetHolsteredItem) self "Holster" "SnapToTarget" "SnapToTarget" "KeepRelative" true)
      (Variables|Default|SetHasItem true))))

(event Custom|Can%20Hold
  ;[1 1 1] Ska funka egentligen men slutade göra det...
  (Utilities|FlowControl|Delay 1.0)
  (Utilities|FlowControl|DoOnce false) ; enters at Reset
)

(fn ConstructionScript)