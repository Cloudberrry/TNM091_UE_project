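; Clock Blueprint that animates second, minute and hour hands by rotating SecSphere, MinSphere and HourSphere.
; Tick drives three chained Delays of a second, a minute and an hour, each followed by a six-degree negative roll step on its sphere.
; Timing relies on Delay ignoring retriggers while pending, so it is approximate and never reads real time.
; The hour hand uses the same step size as the others.
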(event EventTick
  (params (DeltaSeconds :type Float%20%28single-precision%29))
  (bind _secsphere (Variables|Default|GetSecSphere))
  (bind _minsphere (Variables|Default|GetMinSphere))
  (bind _hoursphere (Variables|Default|GetHourSphere))
  (bind _relativerotation (Variables|/Script/Engine.SceneComponent|GetRelativeRotation _secsphere))
  (bind _relativerotation_2 (Variables|/Script/Engine.SceneComponent|GetRelativeRotation _hoursphere))
  (bind _relativerotation_3 (Variables|/Script/Engine.SceneComponent|GetRelativeRotation _minsphere))
  (Utilities|FlowControl|Delay 1.0)
  (Transformation|SetRelativeRotation _secsphere (Math|Rotator|MakeRotator (+ (.roll _relativerotation) -6.0) (.pitch _relativerotation) (.yaw _relativerotation)) false false)
  (Utilities|FlowControl|Delay 6e+01)
  (Transformation|SetRelativeRotation _minsphere (Math|Rotator|MakeRotator (+ (.roll _relativerotation_3) -6.0) (.pitch _relativerotation_3) (.yaw _relativerotation_3)) false false)
  (Utilities|FlowControl|Delay 3.6e+03)
  (Transformation|SetRelativeRotation _hoursphere (Math|Rotator|MakeRotator (+ (.roll _relativerotation_2) -6.0) (.pitch _relativerotation_2) (.yaw _relativerotation_2)) false false))

(fn ConstructionScript)